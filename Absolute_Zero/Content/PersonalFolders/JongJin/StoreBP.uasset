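; StoreBP is an actor with a static mesh and a capsule trigger that highlights the mesh while a RevenantPlayerCharacter overlaps it.
; Capsule begin and end overlap toggle Render CustomDepth on the mesh.
; Both handlers also turn on physics simulation on the player character's mesh, and neither turns it off.
; BeginPlay, Tick, actor overlap and the construction script are empty, and no store logic is present.
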(event OnComponentBeginOverlap(CapsuleCollision)
  (params (OverlappedComponent :type Primitive%20Component%20Object%20Reference) (OtherActor :type Actor%20Object%20Reference) (OtherComp :type Primitive%20Component%20Object%20Reference) (OtherBodyIndex :type Integer) (bFromSweep :type Boolean) (SweepResult :type Hit%20Result%20Structure%20%28by%20ref%29))
  (bind _asrevenant_player_character (Utilities|Casting|CastToRevenantPlayerCharacter OtherActor))
  (Physics|SetSimulatePhysics (Variables|/Script/Engine.Character|GetMesh _asrevenant_player_character) true)
  (Rendering|SetRenderCustomDepth (Variables|Default|Getstaticmash) true))

(event OnComponentEndOverlap(CapsuleCollision)
  (params (OverlappedComponent :type Primitive%20Component%20Object%20Reference) (OtherActor :type Actor%20Object%20Reference) (OtherComp :type Primitive%20Component%20Object%20Reference) (OtherBodyIndex :type Integer))
  (bind _asrevenant_player_character (Utilities|Casting|CastToRevenantPlayerCharacter OtherActor))
  (Physics|SetSimulatePhysics (Variables|/Script/Engine.Character|GetMesh _asrevenant_player_character) true)
  (Rendering|SetRenderCustomDepth (Variables|Default|Getstaticmash) false))

(event EventBeginPlay)

(event Collision|EventActorBeginOverlap
  (params (OtherActor :type Actor%20Object%20Reference)))

(event EventTick
  (params (DeltaSeconds :type Float%20%28single-precision%29)))

(fn ConstructionScript)