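; BPC_Character_DamageSystem is a character damage component that tracks health and death state.
; TakeDamage subtracts the amount in a DamageInfo struct from Health, then either sets IsDead and calls OnDeath, or calls OnDamageResponse with the struct's response value.
; It always returns true and has no guard against damage after death; the event graph holds only disabled default nodes.
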(event EventBeginPlay
  (|CallParentFunction) ; This node is disabled and will not be called.\nDrag off pins to build functionality.
)

(event EventTick
  (params (DeltaSeconds :type Float%20%28single-precision%29))
  (|CallParentFunction DeltaSeconds) ; This node is disabled and will not be called.\nDrag off pins to build functionality.
)

(fn TakeDamage
  (params (DamageInfo :type S%20Damage%20Info%20Structure))
  (bind (_amount _damagetype _damageresponse) (Utilities|Struct|BreakS_DamageInfo DamageInfo))
  (bind _output_get (Variables|Default|SetHealth (- (Variables|Default|GetHealth) _amount)))
  (if (<= _output_get 0.0)
    (Variables|Default|SetIsDead true)
    (Default|CallOnDeath)
    (else
      (Default|CallOnDamageResponse _damageresponse)))
  (return true))