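; BP_EnergyShield is an energy shield actor that switches on and off, with its Area collision set to ignore the Alpha actor when moving.
; Activate enables query-only collision and expands the shield, while Deactivate disables collision and shrinks it; Init starts it hidden at zero scale.
; One ShrinkTimeline drives the particle system's scale, playing forward to shrink and in reverse to expand.
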(event OnComponentBeginOverlap(Area)
  (params (OverlappedComponent :type Primitive%20Component%20Object%20Reference) (OtherActor :type Actor%20Object%20Reference) (OtherComp :type Primitive%20Component%20Object%20Reference) (OtherBodyIndex :type Integer) (bFromSweep :type Boolean) (SweepResult :type Hit%20Result%20Structure%20%28by%20ref%29)))

(event Custom|Activate
  (Collision|SetCollisionEnabled (Variables|Default|GetArea) "QueryOnly")
  (CallFunction|ExpandShield))

(event Custom|Deactivate
  (Collision|SetCollisionEnabled (Variables|Default|GetArea) "NoCollision")
  (CallFunction|ShrinkShield))

(event Custom|ShrinkShield
  (bind _scale (Timeline|ShrinkTimeline PlayFromStart)
    (:Update
      (Transformation|SetRelativeScale3D (Variables|Default|GetParticleSystem) (Math|Conversions|ToVector(Float) _scale)))))

(event Custom|ExpandShield
  (bind _scale (Timeline|ShrinkTimeline ReverseFromEnd)
    (:Update
      (Transformation|SetRelativeScale3D (Variables|Default|GetParticleSystem) (Math|Conversions|ToVector(Float) _scale)))))

(event Custom|Init
  (Collision|SetCollisionEnabled (Variables|Default|GetArea) "NoCollision")
  (Transformation|SetRelativeScale3D (Variables|Default|GetParticleSystem) "0, 0, 0"))

(event Collision|EventActorBeginOverlap
  (params (OtherActor :type Actor%20Object%20Reference)))

(event EventTick
  (params (DeltaSeconds :type Float%20%28single-precision%29)))

(event EventBeginPlay
  (bind _returnvalue (Actor|GetActorOfClass "/Game/PersonalFolders/BaekSeungjun/Bose/Alpha/Alpha.Alpha_C"))
  (Collision|IgnoreActorwhenMoving (Variables|Default|GetArea) _returnvalue true))

(fn ConstructionScript)