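; Damage component that manages its owner's health, healing, blocking and death.
; TakeDamage branches through CanBeDamage on death, invincibility and block state, then fires blocked, damage-response or death callbacks.
; Non-lethal hits show a hit marker; kills show a skull widget and grant EXP to the first RevenantPlayerCharacter found.
; Owners listed in BossArray get a boss-state widget, updated on Tick and removed at zero health.
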(event EventTick
  (params (DeltaSeconds :type Float%20%28single-precision%29))
  (bind _health (Variables|Default|GetHealth))
  (bind _getwidget (Variables|Default|GetGetWidget))
  (Class|IFBossInfo|BossInfo(Message) _getwidget (Components|GetOwner) _health (Variables|Default|GetmaxHealth))
  (if (<= _health 0.0)
    (Widget|RemovefromParent _getwidget)))

(event EventBeginPlay
  (for _array_element (Variables|Default|GetBossArray)
    (if (== _array_element (Components|GetOwner))
      (bind _as플레이어_컨트롤러 (Utilities|Casting|CastToPlayerController (Game|GetPlayerController 0)))
      (bind _returnvalue (UserInterface|CreateWidget "/Game/PersonalFolders/SeoJemin/GameUI/WaveSystme/WB_BossState.WB_BossState_C" _as플레이어_컨트롤러))
      (bind _output_get (Variables|Default|SetGetWidget _returnvalue))
      (UserInterface|Viewport|AddtoViewport _returnvalue 0))))

(fn Heal
  (params (Amount :type Float%20%28double-precision%29))
  (if (not (Variables|Default|GetIsDead))
    (bind _output_get (Variables|Default|SetHealth (Math|Float|Clamp(Float) (+ Amount (Variables|Default|GetHealth)) 0.0 (Variables|Default|GetmaxHealth))))
    (return _output_get)))

(fn TakeDamage
  (params (DamageInfo :type S%20Damage%20Info%20Structure))
  (bind (_amount _damagetype _damageresponse _shoulddamageinvincible _canbeblocked _canbeparried) (Utilities|Struct|BreakS_DamageInfo DamageInfo))
  (Utilities|CanbeDamage _shoulddamageinvincible _canbeblocked
    (:BlockedDamage
      (Default|CallOnBlocked _canbeparried)
      (return false))
    (:DoDamage
      (bind _output_get (Variables|Default|SetHealth (- (Variables|Default|GetHealth) _amount)))
      (if (<= _output_get 0.0)
        (Variables|Default|SetIsDead true)
        (Default|CallOnDeath)
        (bind _returnvalue (UserInterface|CreateWidget "/Game/PersonalFolders/ShinDongjun/Widgets/BP_KillSkull.BP_KillSkull_C" (Game|GetPlayerController 0)))
        (UserInterface|Viewport|AddtoViewport _returnvalue 0)
        (bind _outactors (Actor|GetAllActorsOfClass "/Game/PersonalFolders/ShinDongjun/RevenantPlayerCharacter.RevenantPlayerCharacter_C"))
        (Default|GainEXP (Utilities|Array|Get(acopy) _outactors) (Variables|Default|GetEXP))
        (return true)
        (elif true
          (Default|CallOnDamageResponse _damageresponse)
          (bind _returnvalue_2 (UserInterface|CreateWidget "/Game/PersonalFolders/ShinDongjun/Widgets/BP_HitMarker.BP_HitMarker_C"))
          (UserInterface|Viewport|AddtoViewport _returnvalue_2 0)
          (return true))))
    (:NoDamage
      (return false))))