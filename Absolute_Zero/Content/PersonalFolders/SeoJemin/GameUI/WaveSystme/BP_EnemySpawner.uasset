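; Wave-system enemy spawner that holds a queue of enemy classes and spawns them as AI pawns at its own location.
; Adding to the queue triggers an immediate spawn attempt, and a looping timer keeps draining it front first.
; Spawned pawns get a destroy binding, and a defeat handler notifies BP_ThirdPersonGameMode.
; The game mode's end-wave event sets IsOn once the next wave reaches RoundActivated, though spawning here never checks it.
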(event Custom|OnEnemyDefeated
  (params (DestroyedActor :type Actor%20Object%20Reference))
  (bind _asbp_third_person_game_mode (Utilities|Casting|CastToBP_ThirdPersonGameMode (Game|GetGameMode)))
  (Default|OnEnemyDefeated _asbp_third_person_game_mode))

(event Custom|TryToSpawn
  (CallFunction|SpawnEnemy))

(event Custom|OnEndWave
  (Variables|Default|SetIsOn (>= (+ (Variables|/Game/PersonalFolders/SeoJemin/GameUI/WaveSystme/BP_ThirdPersonGameMode.BP_ThirdPersonGameMode_C|GetWaveNumber (Variables|Default|GetAs%20BP%20Third%20Person%20Game%20Mode)) 1) (Variables|Default|GetRoundActivated))))

(event EventBeginPlay
  (Utilities|Time|SetTimerbyEvent (delegate Custom|TryToSpawn) 2.0 true)
  (bind _asbp_third_person_game_mode (Utilities|Casting|CastToBP_ThirdPersonGameMode (Game|GetGameMode)))
  (bind _output_get (Variables|Default|SetAs%20BP%20Third%20Person%20Game%20Mode _asbp_third_person_game_mode))
  (EventDispatchers|BindEventtoOnEndWave _output_get (delegate Custom|OnEndWave)))

(fn ConstructionScript)

(fn SpawnEnemy
  (if (Utilities|Array|IsValidIndex (Variables|Default|GetEnemyQueue))
    (bind _returnvalue (AI|SpawnAIFromClass (Utilities|Array|Get(acopy) (Variables|Default|GetEnemyQueue)) 0 (Math|Transform|TransformLocation (Transformation|GetActorTransform) "0, 0, 0") "0, 0, 0" true 0))
    (Game|BindEventtoOnDestroyed _returnvalue (EventDispatchers|CreateEvent :!event Custom|OnEnemyDefeated))
    (Utilities|Array|RemoveIndex (Variables|Default|GetEnemyQueue))
    (return true)
    (else
      (return false))))

(fn AddEnemytoQueue
  (params (EnemyClass :type Enemy%20BP%20Class%20Reference%20%28by%20ref%29))
  (Utilities|Array|Add (Variables|Default|GetEnemyQueue) EnemyClass)
  (if (Utilities|Array|IsValidIndex (Collision|GetOverlappingActors (Variables|Default|GetSphere) "/Game/PersonalFolders/BaekSeungjun/Bose/Enemy_BP.Enemy_BP_C" :!class /Script/Engine.PrimitiveComponent))
    _
    (else
      _))
  (CallFunction|SpawnEnemy))