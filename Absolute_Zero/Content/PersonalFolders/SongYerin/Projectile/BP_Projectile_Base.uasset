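; Base projectile Blueprint that flies at a configurable speed and gravity, optionally aimed at a Target actor.
; Construction applies movement settings and enables the homing flag, but the node assigning the homing target component never runs.
; BeginPlay ignores collision with the instigator or owner and points velocity at the Target once.
; On hit, it calls the OnProjectileimpact dispatcher, plays impact effect and sound, then destroys itself.
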(event OnComponentHit(BoxCollision)
  (params (HitComponent :type Primitive%20Component%20Object%20Reference) (OtherActor :type Actor%20Object%20Reference) (OtherComp :type Primitive%20Component%20Object%20Reference) (NormalImpulse :type Vector :default "0, 0, 0") (Hit :type Hit%20Result%20Structure%20%28by%20ref%29))
  (bind _location (Collision|BreakHitResult Hit))
  (Default|CallOnProjectileimpact OtherActor Hit)
  (Effects|SpawnEmitteratLocation (Variables|Effects|GetImpact%20Effect) _location)
  (Audio|PlaySoundatLocation (Variables|sounds|GetImpact%20Sound) _location "0, 0, 0" 1.0 1.0 0.0 0 0 0 0)
  (Actor|DestroyActor))

(event Custom|RotatetoTarget
  (Variables|/Script/Engine.MovementComponent|SetVelocity (Variables|Default|GetProjectileMovement) (* (Math|Vector|GetUnitDirection(Vector) (Transformation|GetActorLocation) (Transformation|GetActorLocation (Variables|Target|Gettarget))) (Variables|Projectilesettings|Getspeed))))

(event EventBeginPlay
  (bind _returnvalue (Game|GetInstigator))
  (Collision|IgnoreActorwhenMoving (Variables|Default|GetBoxCollision) (select (Utilities|IsValid _returnvalue) _returnvalue (Components|GetOwner)) true)
  (Variables|Target|Gettarget
    (:then
      (CallFunction|RotatetoTarget))
    (:else)))

(fn ConstructionScript
  (bind _projectilemovement (Variables|Default|GetProjectileMovement))
  (Variables|/Script/Engine.ProjectileMovementComponent|SetInitialSpeed _projectilemovement (Variables|Projectilesettings|Getspeed))
  (Variables|/Script/Engine.ProjectileMovementComponent|SetMaxSpeed _projectilemovement (Variables|Projectilesettings|Getspeed))
  (Variables|/Script/Engine.ProjectileMovementComponent|SetProjectileGravityScale _projectilemovement (Variables|Projectilesettings|Getgravity))
  (Variables|Target|Gettarget
    (:then
      (if (Variables|Default|GetIsHoming)
        (Variables|/Script/Engine.ProjectileMovementComponent|SetbIsHomingProjectile _projectilemovement true)))
    (:else)))