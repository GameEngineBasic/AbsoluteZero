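; Skill 2 projectile that signals buff completion on overlap and carries helpers for changing character movement speed.
; Overlap runs the parent handler, makes an Enemy tag check with no effect, then calls CompleteBuffs.
; Uncalled here, custom events slow or restore the player's walk speed, while PlayBuff and EndBuff raise or lower that of Enemys.
; Effect spawning, attachment and self-destruction are unwired, and playBuff is empty.
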(event Custom|playBuff)

(event Custom|PlaySpeedDebuff
  (bind _as캐릭터 (Utilities|Casting|CastToCharacter (Game|Player|GetPlayerPawn 0)))
  (Variables|/Script/Engine.CharacterMovementComponent|SetMaxWalkSpeed (Variables|/Script/Engine.Character|GetCharacterMovement _as캐릭터) 2e+02))

(event Custom|Re
  (bind _as캐릭터 (Utilities|Casting|CastToCharacter (Game|Player|GetPlayerPawn 0)))
  (Variables|/Script/Engine.CharacterMovementComponent|SetMaxWalkSpeed (Variables|/Script/Engine.Character|GetCharacterMovement _as캐릭터) 6e+02)
  (Components|Movement|StopMovementImmediately (Variables|/Script/Engine.Character|GetCharacterMovement _as캐릭터)))

(event Collision|EventActorBeginOverlap
  (params (OtherActor :type Actor%20Object%20Reference))
  (|CallParentFunction OtherActor)
  (for _array_element (Collision|GetOverlappingActors 0 :!class /Script/Engine.Actor)
    (if (Actor|ActorHasTag "Enemy")
      _))
  (Default|CallCompleteBuffs))

(event EventTick
  (params (DeltaSeconds :type Float%20%28single-precision%29))
  (|CallParentFunction DeltaSeconds) ; 지금 이 노드는 비활성 상태입니다. \n핀을 끌어서 다른 노드를 연결하면 활성화됩니다.
)

(fn ConstructionScript
  (|CallParentFunction))

(fn PlayBuff
  (bind _as캐릭터 (Utilities|Casting|CastToCharacter (Variables|Default|GetEnemys)))
  (Variables|/Script/Engine.CharacterMovementComponent|SetMaxWalkSpeed (Variables|/Script/Engine.Character|GetCharacterMovement _as캐릭터) 6e+02))

(fn EndBuff
  (bind _as캐릭터 (Utilities|Casting|CastToCharacter (Variables|Default|GetEnemys)))
  (Variables|/Script/Engine.CharacterMovementComponent|SetMaxWalkSpeed (Variables|/Script/Engine.Character|GetCharacterMovement _as캐릭터) 3e+02))